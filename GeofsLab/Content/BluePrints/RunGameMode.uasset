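; Game mode for an endless-runner level that shows the run HUD and builds the starting track.
; On BeginPlay it creates the RunHUD widget and spawns an initial run of floor tiles.
; AddFloorTile picks a random class from the Floortiles array, spawns it at NextSpawnPoint, then takes that tile's attach transform as the next spawn point, chaining tiles end to end.
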(event EventBeginPlay
  (bind _returnvalue (UserInterface|CreateWidget "/Game/UMG/RunHUD.RunHUD_C"))
  (UserInterface|Viewport|AddtoViewport _returnvalue 0)
  (for _index (range 0 9)
    (CallFunction|AddFloorTile)))

(fn ConstructionScript)

(fn AddFloorTile
  (bind _floortiles (Variables|Default|GetFloortiles))
  (bind _returnvalue (Game|SpawnActorfromClass (Utilities|Array|Get(acopy) _floortiles (Math|Random|RandomIntegerinRange 0 (Utilities|Array|LastIndex _floortiles))) (Variables|Default|GetNextSpawnPoint) "Undefined" 0 0))
  (bind _asbp_floortile (Utilities|Casting|CastToBP_Floortile _returnvalue))
  (bind _attach_transform (Default|GetAttachTransform _asbp_floortile))
  (Variables|Default|SetNextSpawnPoint _attach_transform))